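; BP_Tank is a player-controlled tank Blueprint that handles camera rotation and firing input.
; On BeginPlay it passes its Barrel and TankTurret components to setter functions defined outside this graph.
; Mouse X yaws a scene component and Mouse Y pitches the spring arm, splitting the rotation axes across two components.
; The Fire action calls a Fire function whose logic is also defined elsewhere.
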(event EventBeginPlay
  (Class|TankPawn|SetBarrelRefrence (Variables|Default|GetBarrel))
  (Class|TankPawn|SetTurretRefrence (Variables|Default|GetTankTurret)))

(event Collision|EventActorBeginOverlap
  (params (OtherActor :type Actor%20Object%20Reference)))

(event EventTick
  (params (DeltaSeconds :type Float%20%28single-precision%29)))

(event Input|ActionEvents|InputActionFire
  (params (Key :type Key%20Structure))
  (:Pressed
    (Class|TankPawn|Fire)))

(event Input|AxisEvents|InputAxisMouseX
  (params (AxisValue :type Float%20%28single-precision%29))
  (Transformation|AddLocalRotation (Variables|Default|GetScene) (Math|Rotator|MakeRotator 0.0 0.0 (* AxisValue 1.2)) false false))

(event Input|AxisEvents|InputAxisMouseY
  (params (AxisValue :type Float%20%28single-precision%29))
  (Transformation|AddLocalRotation (Variables|Default|GetSpringArm) (Math|Rotator|MakeRotator 0.0 (* AxisValue 1.2) 0.0) false false))

(fn ConstructionScript)